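; Test spline actor that places small cube markers at even intervals along its spline.
; The construction script divides the spline length by DevideCount, adds a static mesh component at each distance, and aligns it to the spline's rotation.
; MeshVisible controls whether the cubes show in game, and the spline length is printed for debugging.
; The event graph holds no logic.
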(event EventBeginPlay)

(event Collision|EventActorBeginOverlap
  (params (OtherActor :type Actor%20Object%20Reference)))

(event EventTick
  (params (DeltaSeconds :type Float%20%28single-precision%29)))

(fn ConstructionScript
  (bind _spline (Variables|Default|GetSpline))
  (bind _spline_2 (Variables|Default|GetSpline))
  (bind _returnvalue (Spline|GetSplineLength _spline_2))
  (Development|PrintString (Utilities|String|ToString(Float) _returnvalue) true true "(R=0.000000,G=0.660000,B=1.000000,A=1.000000)" 1e+01)
  (for _index (range 0 (Variables|Default|GetDevideCount))
    (bind _returnvalue_2 (AddComponent|AddStaticMeshComponent false (Math|Transform|MakeTransform (Math|Transform|InverseTransformLocation (Transformation|GetActorTransform) (Spline|GetLocationatDistanceAlongSpline _spline (* _index (/ _returnvalue (Math|Conversions|ToFloat(Integer) (Variables|Default|GetDevideCount)))) "World")))))
    (Components|StaticMesh|SetStaticMesh _returnvalue_2 "/Game/Etc/Cube_2.Cube_2")
    (Transformation|SetWorldRotation _returnvalue_2 (Spline|GetRotationatDistanceAlongSpline _spline (* _index (/ _returnvalue (Math|Conversions|ToFloat(Integer) (Variables|Default|GetDevideCount)))) "World") false false)
    (Transformation|SetWorldScale3D _returnvalue_2 "0.100000,0.100000,0.100000")
    (Development|SetHiddeninGame _returnvalue_2 (not (Variables|Default|GetMeshVisible)) false)))